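; BP_LandMine is a land mine trap Blueprint that supplies the sound and visual effects for its alert and explosion.
; Custom events start a looping click alarm as a 2D sound, store it in AlarmSound, and stop it.
; A third event plays an explosion sound and particle emitter at the actor's transform.
; Overlap, tick and begin play are disabled, and nothing in this graph calls these events.
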(event EventBeginPlay)

(event Collision|EventActorBeginOverlap
  (params (OtherActor :type Actor%20Object%20Reference)))

(event EventTick
  (params (DeltaSeconds :type Float%20%28single-precision%29)))

(event EventMakeAlertSound
  (bind _returnvalue (Audio|SpawnSound2D "/Engine/VREditor/Sounds/UI/Click_on_Button_Loop_Cue.Click_on_Button_Loop_Cue" 1.0 1.0 0.0 0))
  (Variables|Default|SetAlarmSound _returnvalue))

(event EventStopAlertSound
  (Audio|Components|Audio|Stop (Variables|Default|GetAlarmSound)))

(event EventMakeExplodeEffects
  (bind _returnvalue (Transformation|GetActorTransform))
  (bind (_location _rotation _scale) (Math|Transform|BreakTransform _returnvalue))
  (Audio|SpawnSoundatLocation "/Game/StarterContent/Audio/Explosion01.Explosion01" (Transformation|GetActorLocation) "0, 0, 0" 1.0 1.0 0.0 0 0)
  (Effects|SpawnEmitteratLocation "/Game/StarterContent/Particles/P_Explosion.P_Explosion" _location _rotation _scale))

(fn ConstructionScript)